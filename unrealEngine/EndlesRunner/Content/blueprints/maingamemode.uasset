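; Game mode that builds an endless-runner style ground track out of randomly chosen segments.
; BeginPlay spawns an initial run of eight segments through the Newgroundcreate event.
; Each call spawns a random class from the Zeminler array at the stored location, then takes that groundbp's Newground component transform as the next spawn point, chaining tiles end to end.
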(event Custom|newgroundcreate
  (bind _zeminler (Variables|Default|Getzeminler))
  (bind _returnvalue (Game|SpawnActorfromClass (Utilities|Array|Get(acopy) _zeminler (Math|Random|RandomIntegerinRange 0 (Utilities|Array|LastIndex _zeminler))) (Variables|Default|Getnewgroundlocation) "Undefined" 0 0))
  (bind _asgroundbp (Utilities|Casting|CastTogroundbp _returnvalue))
  (Variables|Default|Setnewgroundlocation (Transformation|GetWorldTransform (Variables|/Game/blueprints/groundbp.groundbp_C|Getnewground _asgroundbp))))

(event EventBeginPlay
  (for _index (range 0 7)
    (CallFunction|Newgroundcreate)))

(fn ConstructionScript)