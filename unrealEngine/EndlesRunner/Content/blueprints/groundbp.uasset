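; Ground segment Blueprint for what appears to be an endless runner, with side walls that kill the main character on hit.
; The construction script always spawns barriers and, one time in three, coins, as child actors at random points in the Spawnpointer box.
; When the character overlaps Lastcollision, the game mode creates the next ground and this segment destroys itself after a delay.
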(event OnComponentBeginOverlap(lastcollision)
  (params (OverlappedComponent :type Primitive%20Component%20Object%20Reference) (OtherActor :type Actor%20Object%20Reference) (OtherComp :type Primitive%20Component%20Object%20Reference) (OtherBodyIndex :type Integer) (bFromSweep :type Boolean) (SweepResult :type Hit%20Result%20Structure%20%28by%20ref%29))
  (Utilities|Casting|CastTomaincharacter OtherActor)
  (bind _asmaingamemode (Utilities|Casting|CastTomaingamemode (Game|GetGameMode)))
  (Default|Newgroundcreate _asmaingamemode)
  (Utilities|FlowControl|Delay 1e+01)
  (Actor|DestroyActor))

(event OnComponentHit(rightwall)
  (params (HitComponent :type Primitive%20Component%20Object%20Reference) (OtherActor :type Actor%20Object%20Reference) (OtherComp :type Primitive%20Component%20Object%20Reference) (NormalImpulse :type Vector :default "0, 0, 0") (Hit :type Hit%20Result%20Structure%20%28by%20ref%29))
  (bind _asmaincharacter (Utilities|Casting|CastTomaincharacter OtherActor))
  (Default|Death _asmaincharacter))

(event OnComponentHit(leftwall)
  (params (HitComponent :type Primitive%20Component%20Object%20Reference) (OtherActor :type Actor%20Object%20Reference) (OtherComp :type Primitive%20Component%20Object%20Reference) (NormalImpulse :type Vector :default "0, 0, 0") (Hit :type Hit%20Result%20Structure%20%28by%20ref%29))
  (bind _asmaincharacter (Utilities|Casting|CastTomaincharacter OtherActor))
  (Default|Death _asmaincharacter))

(event EventBeginPlay)

(event Collision|EventActorBeginOverlap
  (params (OtherActor :type Actor%20Object%20Reference)))

(event EventTick
  (params (DeltaSeconds :type Float%20%28single-precision%29)))

(fn ConstructionScript
  (switch int (Math|Random|RandomIntegerinRange 0 2)
    (:0
      (CallFunction|Barrierspawn :!label _label))
    (:1
      (goto _label))
    (:2
      (CallFunction|Coinspawn)
      (CallFunction|Barrierspawn))))

(fn Coinspawn
  (bind _spawnpointer (Variables|Default|Getspawnpointer))
  (for _index (range 0 (Math|Random|RandomIntegerinRange 4 8))
    (AddComponent|AddChildActorComponent false (Math|Transform|MakeTransform (Math|Random|RandomPointinBoundingBox (Variables|/Script/Engine.SceneComponent|GetRelativeLocation _spawnpointer) (Variables|/Script/Engine.BoxComponent|GetBoxExtent _spawnpointer)) "0, 0, 0" "1,1,1"))))

(fn Barrierspawn
  (bind _spawnpointer (Variables|Default|Getspawnpointer))
  (for _index (range 0 (Math|Random|RandomIntegerinRange 1 2))
    (AddComponent|AddChildActorComponent true (Math|Transform|MakeTransform (Math|Random|RandomPointinBoundingBox (Transformation|GetWorldLocation _spawnpointer) (Variables|/Script/Engine.BoxComponent|GetBoxExtent _spawnpointer)) "0, 0, 0" "1,1,1"))))